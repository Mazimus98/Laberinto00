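; BP_boton2 is a pressure button that controls raisable walls (BP_ParedElevadiza) while something overlaps its Box.
; On begin or end overlap, it finds all walls in the level and calls BotonPresionado or BotonLiberado on those whose NumeroPuerta matches its NumeroDeBoton.
; A timeline slides the button mesh in and reverses it on release.
; Disconnected leftover logic targets BP_Puerta3 doors.
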(event `self.Box.OnComponentBeginOverlap`
  (params (OverlappedComponent :type "PrimitiveComponent Object Reference") (OtherActor :type "Actor Object Reference") (OtherComp :type "PrimitiveComponent Object Reference") (OtherBodyIndex :type Integer) (bFromSweep :type Boolean) (SweepResult :type "HitResult Structure (by ref)"))
  (if true
    (`|ExecutionSequence`
      (:`then_0`
        (bind _outactors (`GameplayStatics.GetAllActorsOfClass` "/Game/mecanicas/Paredes/BP_ParedElevadiza.BP_ParedElevadiza_C"))
        (for _array_element _outactors
          (if (== (`/Game/mecanicas/Paredes/BP_ParedElevadiza.numeroPuerta` _array_element) (`self.NumeroDeBoton`))
            (`/Game/mecanicas/Paredes/BP_ParedElevadiza.BotonPresionado` _array_element))))
      (:`then_1`
        (bind (_direction _newtrack_0) (`Timeline|Timeline_0` :!label _label)
          (:`Update`
            (`SceneComponent.K2_SetRelativeLocation` (`self.StaticMesh`) (`KismetMathLibrary.MakeVector` 10.0 (`KismetMathLibrary.Lerp` 0.0 19.0 _newtrack_0)) false false)))))))

(event `self.ReceiveActorEndOverlap`
  (params (OtherActor :type "Actor Object Reference")))

(event `self.Box.OnComponentEndOverlap`
  (params (OverlappedComponent :type "PrimitiveComponent Object Reference") (OtherActor :type "Actor Object Reference") (OtherComp :type "PrimitiveComponent Object Reference") (OtherBodyIndex :type Integer))
  (`|ExecutionSequence`
    (:`then_0`
      (bind _outactors (`GameplayStatics.GetAllActorsOfClass` "/Game/mecanicas/Paredes/BP_ParedElevadiza.BP_ParedElevadiza_C"))
      (for _array_element _outactors
        (if (== (`/Game/mecanicas/Paredes/BP_ParedElevadiza.numeroPuerta` _array_element) (`self.NumeroDeBoton`))
          (`/Game/mecanicas/Paredes/BP_ParedElevadiza.BotonLiberado` _array_element))))
    (:`then_1`
      (goto _label :!via `Reverse`))))

(fn `UserConstructionScript`)
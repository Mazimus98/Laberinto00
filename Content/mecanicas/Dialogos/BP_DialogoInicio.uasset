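; BP_DialogoInicio is a world actor that shows floating dialogue text when the first-person player comes near.
; Overlapping ActivadorDialogo with BP_PrimeraPersona makes TextoDialogo visible, and leaving it hides the text again.
; On entry the text turns to face the player's mesh on yaw only, so it stays upright and does not track further movement.
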(event `self.activadorDialogo.OnComponentBeginOverlap`
  (params (OverlappedComponent :type "PrimitiveComponent Object Reference") (OtherActor :type "Actor Object Reference") (OtherComp :type "PrimitiveComponent Object Reference") (OtherBodyIndex :type Integer) (bFromSweep :type Boolean) (SweepResult :type "HitResult Structure (by ref)"))
  (bind _asbp_primera_persona (cast `/Game/ThirdPerson/Blueprints/BP_PrimeraPersona` OtherActor))
  (bind (_returnvalue_roll _returnvalue_pitch _returnvalue_yaw) (`KismetMathLibrary.BreakRotator` (`KismetMathLibrary.FindLookAtRotation` (`SceneComponent.K2_GetComponentLocation` (`self.textoDialogo`)) (`SceneComponent.K2_GetComponentLocation` (`Character.Mesh` _asbp_primera_persona)))))
  (`SceneComponent.K2_SetWorldRotation` (`self.textoDialogo`) (`KismetMathLibrary.MakeRotator` 0.0 0.0 _returnvalue_yaw) false false)
  (`SceneComponent.SetVisibility` (`self.textoDialogo`) true false))

(event `self.activadorDialogo.OnComponentEndOverlap`
  (params (OverlappedComponent :type "PrimitiveComponent Object Reference") (OtherActor :type "Actor Object Reference") (OtherComp :type "PrimitiveComponent Object Reference") (OtherBodyIndex :type Integer))
  (cast `/Game/ThirdPerson/Blueprints/BP_PrimeraPersona` OtherActor)
  (`SceneComponent.SetVisibility` (`self.textoDialogo`) false false))

(fn `UserConstructionScript`)
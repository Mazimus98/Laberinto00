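; BP_PlataformaParedMovediza3 is a pressure plate that triggers moving walls when a box with a matching code is placed on it.
; An overlapping BP_caja whose CodigoCaja equals CodigoPlataforma calls MoverPared on BP_ParedMovediza3 actors sharing that code, while a Timeline lowers the plate mesh.
; Any end overlap clears EstaPresionado, calls MoverPared on every BP_ParedMovediza3 without checking codes, and reverses the Timeline.
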(event `self.Box.OnComponentBeginOverlap`
  (params (OverlappedComponent :type "PrimitiveComponent Object Reference") (OtherActor :type "Actor Object Reference") (OtherComp :type "PrimitiveComponent Object Reference") (OtherBodyIndex :type Integer) (bFromSweep :type Boolean) (SweepResult :type "HitResult Structure (by ref)"))
  (bind _asbp_caja (cast `/Game/mecanicas/cajas/BP_caja` OtherActor))
  (if (== (`/Game/mecanicas/cajas/BP_caja.codigoCaja` _asbp_caja) (`self.codigoPlataforma`))
    (set `self.estaPresionado?` true)
    (`|ExecutionSequence`
      (:`then_0`
        (bind _outactors (`GameplayStatics.GetAllActorsOfClass` "/Game/mecanicas/Paredes/BP_ParedMovediza3.BP_ParedMovediza3_C"))
        (for _array_element _outactors
          (if (and (== true (`self.estaPresionado?`)) (== (`/Game/mecanicas/Paredes/BP_ParedMovediza3.CodigoPared` _array_element) (`self.codigoPlataforma`)))
            (`/Game/mecanicas/Paredes/BP_ParedMovediza3.MoverPared` _array_element))))
      (:`then_1`
        (bind (_direction _newtrack_0) (`Timeline|Timeline` :!label _label)
          (:`Update`
            (`SceneComponent.K2_SetRelativeLocation` (`self.StaticMesh1`) (`KismetMathLibrary.MakeVector` 10.0 10.0 (`KismetMathLibrary.Lerp` 10.0 5.0 _newtrack_0)) false false)))))))

(event `self.Box.OnComponentEndOverlap`
  (params (OverlappedComponent :type "PrimitiveComponent Object Reference") (OtherActor :type "Actor Object Reference") (OtherComp :type "PrimitiveComponent Object Reference") (OtherBodyIndex :type Integer))
  (set `self.estaPresionado?` false)
  (`|ExecutionSequence`
    (:`then_0`
      (bind _outactors (`GameplayStatics.GetAllActorsOfClass` "/Game/mecanicas/Paredes/BP_ParedMovediza3.BP_ParedMovediza3_C"))
      (for _array_element _outactors
        (`/Game/mecanicas/Paredes/BP_ParedMovediza3.MoverPared` _array_element)))
    (:`then_1`
      (goto _label :!via `Reverse`))))

(fn `UserConstructionScript`)
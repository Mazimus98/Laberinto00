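; BP_PlataformaParedAsesina4 is a pressure plate that triggers BP_ParedAsesina4 killer walls when BP_PrimeraPersona steps on or off it.
; Box overlap begin sets EstaPresionado and calls MoverPared on walls whose CodigoPared matches CodigoPlataforma.
; Overlap end clears the flag and calls MoverPared on every such wall, without checking the code.
; The AnimacionPlataforma timeline lowers the plate mesh while pressed and reverses on release.
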(event `self.Box.OnComponentBeginOverlap`
  (params (OverlappedComponent :type "PrimitiveComponent Object Reference") (OtherActor :type "Actor Object Reference") (OtherComp :type "PrimitiveComponent Object Reference") (OtherBodyIndex :type Integer) (bFromSweep :type Boolean) (SweepResult :type "HitResult Structure (by ref)"))
  (cast `/Game/ThirdPerson/Blueprints/BP_PrimeraPersona` OtherActor)
  (set `self.estaPresionado?` true)
  (`|ExecutionSequence`
    (:`then_0`
      (bind _outactors (`GameplayStatics.GetAllActorsOfClass` "/Game/mecanicas/Paredes/BP_ParedAsesina4.BP_ParedAsesina4_C"))
      (for _array_element _outactors
        (if (and (== (`self.estaPresionado?`) true) (== (`/Game/mecanicas/Paredes/BP_ParedAsesina4.CodigoPared` _array_element) (`self.codigoPlataforma`)))
          (`/Game/mecanicas/Paredes/BP_ParedAsesina4.MoverPared` _array_element))))
    (:`then_1`
      (bind (_direction _newtrack_0) (`Timeline|AnimacionPlataforma` :!label _label)
        (:`Update`
          (`SceneComponent.K2_SetRelativeLocation` (`self.StaticMesh`) (`KismetMathLibrary.MakeVector` -140.0 -110.0 (`KismetMathLibrary.Lerp` -50.0 -70.0 _newtrack_0)) false false))))))

(event `self.Box.OnComponentEndOverlap`
  (params (OverlappedComponent :type "PrimitiveComponent Object Reference") (OtherActor :type "Actor Object Reference") (OtherComp :type "PrimitiveComponent Object Reference") (OtherBodyIndex :type Integer))
  (cast `/Game/ThirdPerson/Blueprints/BP_PrimeraPersona` OtherActor)
  (set `self.estaPresionado?` false)
  (`|ExecutionSequence`
    (:`then_0`
      (bind _outactors (`GameplayStatics.GetAllActorsOfClass` "/Game/mecanicas/Paredes/BP_ParedAsesina4.BP_ParedAsesina4_C"))
      (for _array_element _outactors
        (`/Game/mecanicas/Paredes/BP_ParedAsesina4.MoverPared` _array_element)))
    (:`then_1`
      (goto _label :!via `Reverse`))))

(fn `UserConstructionScript`)
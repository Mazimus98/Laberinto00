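; BP_PisoTrampa is a trap-floor pressure plate that moves the walls paired with it.
; When anything begins overlapping its Box, it sets EstaPresionado and calls MoverPared on every BP_ParedPisoTrampa whose CodigoPared matches NumeroDePlaca.
; End overlap does nothing.
; Disconnected nodes remain for release handling, a plate-lowering timeline, door opening and state-based wall matching.
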(event `self.Box.OnComponentBeginOverlap`
  (params (OverlappedComponent :type "PrimitiveComponent Object Reference") (OtherActor :type "Actor Object Reference") (OtherComp :type "PrimitiveComponent Object Reference") (OtherBodyIndex :type Integer) (bFromSweep :type Boolean) (SweepResult :type "HitResult Structure (by ref)"))
  (set `self.estaPresionado?` true)
  (`|ExecutionSequence`
    (:`then_0`
      (bind _outactors (`GameplayStatics.GetAllActorsOfClass` "/Game/mecanicas/Paredes/BP_ParedPisoTrampa.BP_ParedPisoTrampa_C"))
      (for _array_element _outactors
        (if (== (`/Game/mecanicas/Paredes/BP_ParedPisoTrampa.CodigoPared` _array_element) (`self.NumeroDePlaca`))
          (`/Game/mecanicas/Paredes/BP_ParedPisoTrampa.MoverPared` _array_element))))))

(event `self.Box.OnComponentEndOverlap`
  (params (OverlappedComponent :type "PrimitiveComponent Object Reference") (OtherActor :type "Actor Object Reference") (OtherComp :type "PrimitiveComponent Object Reference") (OtherBodyIndex :type Integer)))

(fn `UserConstructionScript`)
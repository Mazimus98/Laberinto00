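; BP_PlataformaCamuflada is a camouflaged pressure plate that operates hidden walls (BP_ParedEscondida).
; Box overlap sets EstaPresionado, then a nested loop calls MoverPared on walls whose CodigoPared matches CodigoPlataforma, repeated for each closed wall found.
; Ending overlap calls MoverPared on every hidden wall, regardless of code.
; The AnimacionPlataforma timeline moves the mesh along Z on overlap and reverses on exit.
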(event `self.Box.OnComponentBeginOverlap`
  (params (OverlappedComponent :type "PrimitiveComponent Object Reference") (OtherActor :type "Actor Object Reference") (OtherComp :type "PrimitiveComponent Object Reference") (OtherBodyIndex :type Integer) (bFromSweep :type Boolean) (SweepResult :type "HitResult Structure (by ref)"))
  (set `self.estaPresionado?` true)
  (`|ExecutionSequence`
    (:`then_0`
      (bind _outactors (`GameplayStatics.GetAllActorsOfClass` "/Game/mecanicas/Paredes/BP_ParedEscondida.BP_ParedEscondida_C"))
      (for _array_element _outactors
        (if (== (`/Game/mecanicas/Paredes/BP_ParedEscondida.estaCerrada?` _array_element) (`self.estaPresionado?`))
          (for _array_element_2 _outactors
            (if (== (`/Game/mecanicas/Paredes/BP_ParedEscondida.CodigoPared` _array_element_2) (`self.codigoPlataforma`))
              (`/Game/mecanicas/Paredes/BP_ParedEscondida.MoverPared` _array_element_2))))))
    (:`then_1`
      (bind (_direction _newtrack_0) (`Timeline|AnimacionPlataforma` :!label _label)
        (:`Update`
          (`SceneComponent.K2_SetRelativeLocation` (`self.StaticMesh`) (`KismetMathLibrary.MakeVector` 0.0 0.0 _newtrack_0) false false))))))

(event `self.Box.OnComponentEndOverlap`
  (params (OverlappedComponent :type "PrimitiveComponent Object Reference") (OtherActor :type "Actor Object Reference") (OtherComp :type "PrimitiveComponent Object Reference") (OtherBodyIndex :type Integer))
  (set `self.estaPresionado?` false)
  (`|ExecutionSequence`
    (:`then_0`
      (bind _outactors (`GameplayStatics.GetAllActorsOfClass` "/Game/mecanicas/Paredes/BP_ParedEscondida.BP_ParedEscondida_C"))
      (for _array_element _outactors
        (`/Game/mecanicas/Paredes/BP_ParedEscondida.MoverPared` _array_element)))
    (:`then_1`
      (goto _label :!via `Reverse`))))

(fn `UserConstructionScript`)